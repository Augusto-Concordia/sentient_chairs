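; BP_MyFirstActor is a test actor that pushes itself forward periodically and reacts to hits from Characters.
; BeginPlay starts a looping two-second timer that adds an impulse along the actor's forward vector to its primitive component, scaled by ImpulseStrength.
; When hit by a Character, it prints a collision message and turns the ColorSeats parameter red through a dynamic material instance on the hit component.
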(event `self.ReceiveHit`
  (params (MyComp :type "PrimitiveComponent Object Reference") (Other :type "Actor Object Reference") (OtherComp :type "PrimitiveComponent Object Reference") (bSelfMoved :type Boolean) (HitLocation :type "Vector Structure") (HitNormal :type "Vector Structure") (NormalImpulse :type "Vector Structure") (Hit :type "HitResult Structure (by ref)"))
  (bind _ascharacter (cast `Character` Other))
  (if (`KismetSystemLibrary.IsValid` _ascharacter)
    (`KismetSystemLibrary.PrintText` "Collided with FirstPersonCharacter!")
    (bind _returnvalue (`PrimitiveComponent.CreateDynamicMaterialInstance` MyComp 0 null "None"))
    (`MaterialInstanceDynamic.SetVectorParameterValue` _returnvalue "ColorSeats" (struct :`R` 1.0 :`A` 1.0))))

(event `self.ReceiveBeginPlay`
  (`KismetSystemLibrary.K2_SetTimerDelegate` (delegate `Event 2sTrigger`) 2.0 true))

(event `Event 2sTrigger`
  (`PrimitiveComponent.AddImpulse` (`self.GetComponentByClass` "/Script/Engine.PrimitiveComponent") (* (`KismetMathLibrary.GetForwardVector` (`self.K2_GetActorRotation`)) (`self.Impulse Strength`)) "None" false))

(fn `UserConstructionScript`)